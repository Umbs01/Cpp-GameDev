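; Lobby game mode that registers players joining the Lobby level and keeps their shared profile list in sync.
; HandleStartingNewPlayer casts each new controller to the Lobby class, stores it, then triggers its menu creation and initial setup.
; UpdateLobby, when its PlayerNames flag is set, rebuilds the profile list from connected controllers and pushes it back to each one.
; A leftover name-gathering loop is disconnected and never runs.
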(event Custom|UpdateLobby
  (params (PlayerNames :type Boolean))
  (bind _all_playerprofile (Variables|Default|GetAll_PlayerProfile))
  (if PlayerNames
    (Utilities|Array|Clear (Variables|Default|GetAll_PlayerProfile))
    (for _array_element (Variables|Default|GetAllConnectedPlayers)
      (Utilities|Array|Add _all_playerprofile (Variables|/Game/Maps/Lobby/Blueprint/Lobby_C.Lobby_C_C|GetPlayerProfileInfo _array_element))
      (for _array_element_2 _all_playerprofile
        _))
    (for _array_element_3 (Variables|Default|GetAllConnectedPlayers)
      (if PlayerNames
        (Default|UpdatePlayerNames _array_element_3 (Variables|Default|GetAll_PlayerProfile))))))

(event EventHandleStartingNewPlayer
  (params (NewPlayer :type Player%20Controller%20Object%20Reference))
  (bind _returnvalue (Game|GetCurrentLevelName true))
  (switch string _returnvalue
    (:Lobby
      (bind _aslobby_c (Utilities|Casting|CastToLobby_C NewPlayer))
      (Utilities|Array|Add (Variables|Default|GetAllConnectedPlayers) _aslobby_c)
      (Default|CreateLobbyMenu _aslobby_c)
      (Default|InitialSetup _aslobby_c))))

(fn ConstructionScript)