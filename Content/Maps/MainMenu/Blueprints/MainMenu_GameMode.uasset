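; MainMenu_GameMode is the main menu game mode that manages players joining the Lobby level.
; When a new player starts there, it stores their MainMenu_Controller in ConnectedPlayers and triggers lobby menu creation and initial setup on it.
; UpdateLobby, when PlayerNames is set, rebuilds the profile list from those controllers with debug prints, then sends it back to each to update names.
; Disconnected leftover copies of both flows remain in the graph.
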(event Custom|UpdateLobby
  (params (PlayerNames :type Boolean))
  (bind _all_playerprofiles (Variables|Default|GetAll_PlayerProfiles))
  (if PlayerNames
    (Utilities|Array|Clear (Variables|Default|GetAll_PlayerProfiles))
    (for _array_element (Variables|Default|GetConnectedPlayers)
      (Utilities|Array|Add _all_playerprofiles (Variables|/Game/Maps/MainMenu/Blueprints/MainMenu_Controller.MainMenu_Controller_C|GetPlayerProfileInfo _array_element))
      (for _array_element_2 _all_playerprofiles
        (Development|PrintString (Utilities|String|ToString(Text) (Utilities|Struct|BreakS_PlayerProfile _array_element_2)))))
    (for _array_element_3 (Variables|Default|GetConnectedPlayers)
      (if PlayerNames
        (Default|UpdatePlayerNames _array_element_3 (Variables|Default|GetAll_PlayerProfiles))))))

(event EventHandleStartingNewPlayer
  (params (NewPlayer :type Player%20Controller%20Object%20Reference))
  (bind _returnvalue (Game|GetCurrentLevelName true))
  (switch string _returnvalue
    (:Lobby
      (bind _asmain_menu_controller (Utilities|Casting|CastToMainMenu_Controller NewPlayer))
      (Utilities|Array|Add (Variables|Default|GetConnectedPlayers) _asmain_menu_controller)
      (Default|CreateLobbyMenu _asmain_menu_controller)
      (Default|InitialSetup _asmain_menu_controller))))

(fn ConstructionScript)